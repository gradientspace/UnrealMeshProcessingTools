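; BP_MagnaSphere is a sphere actor that is magnetically drawn toward the nearest surface point of a target mesh actor.
; Each Tick queries that point, applies a delta-time-scaled AttractForce impulse toward it, and moves NearestPointComponent onto it.
; It also runs a winding-threshold containment test on the target, swapping between inside and outside materials to show whether its location is within the mesh.
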(event EventBeginPlay)

(event Collision|EventActorBeginOverlap
  (params (OtherActor :type Actor%20Object%20Reference)))

(event EventTick
  (params (DeltaSeconds :type Float%20%28single-precision%29))
  (bind _self self)
  (bind _returnvalue (Transformation|GetActorLocation _self))
  (Utilities|FlowControl|Sequence
    (:then_0
      (bind _nearestmeshworldpoint (Class|DynamicMeshBaseActor|DistancetoPoint (Variables|Default|GetTargetActor) _returnvalue))
      (Physics|AddImpulse (Variables|Debug|GetStaticMeshComponent) (* (Math|Vector|Normalize (- _nearestmeshworldpoint _returnvalue)) (* DeltaSeconds (Variables|Default|GetAttractForce))) "None" false))
    (:then_1
      (bind _nearestmeshworldpoint_2 (Class|DynamicMeshBaseActor|DistancetoPoint (Variables|Default|GetTargetActor) (Transformation|GetActorLocation self)))
      (Transformation|SetRelativeLocation (Variables|Default|GetNearestPointComponent) (Math|Transform|InverseTransformLocation (Transformation|GetActorTransform) _nearestmeshworldpoint_2) false true))
    (:then_2
      (bind _returnvalue_2 (Class|DynamicMeshBaseActor|ContainsPoint (Variables|Default|GetTargetActor) (Transformation|GetActorLocation self) 0.5))
      (if _returnvalue_2
        (Rendering|Material|SetMaterial (Variables|Debug|GetStaticMeshComponent) 0 (Variables|Default|GetInsideMaterial))
        (else
          (Rendering|Material|SetMaterial (Variables|Debug|GetStaticMeshComponent) 0 (Variables|Default|GetOutsideMaterial)))))))

(fn ConstructionScript)