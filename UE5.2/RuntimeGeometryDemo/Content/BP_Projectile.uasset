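; BP_Projectile is a simple projectile actor that flies straight along its forward vector.
; Each Tick it teleports forward by MoveSpeed scaled by delta time, without sweeping for collisions along the path.
; It destroys itself once it has existed for more than five seconds, and contains no overlap or hit logic.
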(event EventBeginPlay)

(event Collision|EventActorBeginOverlap
  (params (OtherActor :type Actor%20Object%20Reference)))

(event EventTick
  (params (DeltaSeconds :type Float%20%28single-precision%29))
  (Transformation|SetActorLocation self (+ (Transformation|GetActorLocation self) (* (Transformation|GetActorForwardVector self) (* DeltaSeconds (Variables|Default|GetMoveSpeed)))) false true)
  (Math|Float|CompareFloat (Actor|GetGameTimeSinceCreation) 5.0
    (:>
      (Actor|DestroyActor))))

(fn ConstructionScript)