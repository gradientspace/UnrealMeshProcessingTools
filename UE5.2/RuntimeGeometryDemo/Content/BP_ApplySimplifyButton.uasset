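; BP_ApplySimplifyButton is an overlap-triggered button actor that simplifies the mesh of a target actor.
; When an actor begins overlapping it, it shows its pressed material and, if SimplifyTargetActor is valid, calls SimplifyMeshToTriCount with half that actor's current triangle count.
; Each new overlap halves the count again, and ending an overlap only restores the not-pressed material.
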(event EventBeginPlay)

(event Collision|EventActorBeginOverlap
  (params (OtherActor :type Actor%20Object%20Reference))
  (Rendering|Material|SetMaterial (Variables|Debug|GetStaticMeshComponent) 0 (Variables|Default|GetPressedMaterial))
  (bind _simplifytargetactor (Variables|Default|GetSimplifyTargetActor)
    (:then
      (bind _returnvalue (Class|DynamicBaseActor|GetTriangleCount _simplifytargetactor))
      (Class|DynamicBaseActor|SimplifyMeshtoTriCount _simplifytargetactor (/ _returnvalue 2)))
    (:else)))

(event EventTick
  (params (DeltaSeconds :type Float%20%28single-precision%29)))

(event Collision|EventActorEndOverlap
  (params (OtherActor :type Actor%20Object%20Reference))
  (Rendering|Material|SetMaterial (Variables|Debug|GetStaticMeshComponent) 0 (Variables|Default|GetNotPressedMaterial)))

(fn ConstructionScript)