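; BP_RotatoSphere is an actor that visualizes nearest-point and containment queries against a target mesh actor as it spins.
; Each Tick rotates the static mesh, with frame-rate-scaled yaw and a fixed per-frame roll.
; It then queries TargetActor at RotatingComponent's position, moving a marker component to the nearest surface point in actor-local space.
; A winding-number inside test switches RotatingComponent between inside and outside materials.
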(event EventBeginPlay)

(event Collision|EventActorBeginOverlap
  (params (OtherActor :type Actor%20Object%20Reference)))

(event EventTick
  (params (DeltaSeconds :type Float%20%28single-precision%29))
  (Utilities|FlowControl|Sequence
    (:then_0
      (Transformation|AddWorldRotation (Variables|Debug|GetStaticMeshComponent) (Math|Rotator|MakeRotator 0.1 0.0 (* DeltaSeconds 1e+02)) false false))
    (:then_1
      (bind _nearestmeshworldpoint (Class|DynamicMeshBaseActor|DistancetoPoint (Variables|Default|GetTargetActor) (Transformation|GetWorldLocation (Variables|Default|GetRotatingComponent))))
      (Transformation|SetRelativeLocation (Variables|Default|GetNearestPointComponent) (Math|Transform|InverseTransformLocation (Transformation|GetActorTransform) _nearestmeshworldpoint) false true))
    (:then_2
      (bind _returnvalue (Class|DynamicMeshBaseActor|ContainsPoint (Variables|Default|GetTargetActor) (Transformation|GetWorldLocation (Variables|Default|GetRotatingComponent)) 0.5))
      (if _returnvalue
        (Rendering|Material|SetMaterial (Variables|Default|GetRotatingComponent) 0 (Variables|Default|GetInsideMaterial))
        (else
          (Rendering|Material|SetMaterial (Variables|Default|GetRotatingComponent) 0 (Variables|Default|GetOutsideMaterial)))))))

(fn ConstructionScript)